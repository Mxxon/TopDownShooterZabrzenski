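; Spider enemy that chases the player, melee attacks in range and dies when its HP runs out.
; BeginPlay loops AIMoveTo while alive, and Tick checks distance to play the attack montage with movement deactivated.
; AnyDamage lowers HP through ClampAngle; at zero it disables collision, increments BP_Soldier_01's Kills and destroys the actor after a delay.
; DamageCharacter applies hit damage to the player but is not called within this Blueprint.
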(event `self.ReceiveBeginPlay`
  ;[1 1 1] Tracking/movement
  (if (`self.IsAlive`) :!label _label
    (`|AIMoveTo` self (0.0 0.0 0.0) (`GameplayStatics.GetPlayerCharacter` 0)
      (:`OnSuccess`
        _)
      (:`OnFail`
        _))
    (`KismetSystemLibrary.Delay` 0.2)
    (goto _label)))

(event `self.ReceiveTick`
  (params (DeltaSeconds :type "Float (single-precision)"))
  (if (and (`self.IsAttackRange`) (`self.IsAlive`) (not (`self.IsAttacking`)))
    (`ActorComponent.Deactivate` (`self.CharacterMovement`))
    (`|PlayMontage` (`self.Mesh`) "/Game/Characters/Enemy_Great_Spider/Animations/SpiderAttack_01.SpiderAttack_01"
      (:`OnCompleted`
        (`ActorComponent.SetActive` (`self.CharacterMovement`) true false)))))

(event `self.ReceiveAnyDamage`
  (params (Damage :type "Float (single-precision)") (DamageType :type "DamageType Object Reference") (InstigatedBy :type "Controller Object Reference") (DamageCauser :type "Actor Object Reference"))
  (bind _output_get (`self.Damage Amount` Damage))
  (if (== _output_get 0.0)
    (`self.DeadAI`)
    (`KismetSystemLibrary.Delay` 2.0)
    (`self.K2_DestroyActor`)))

(fn `Damage Amount`
  (params (B :type "Float (double-precision)"))
  (returns (Output_Get :type "Float (double-precision)"))
  (bind _output_get (set `self.HP` (`KismetMathLibrary.ClampAngle` (- (`self.HP`) B) 0.0 100.0)))
  (return _output_get))

(fn `DamageCharacter`
  (`GameplayStatics.ApplyDamage` (`GameplayStatics.GetPlayerCharacter` 0) (`self.DamagePerHit`)))

(fn `DeadAI`
  (set `self.Dead` true)
  (`MovementComponent.StopMovementImmediately` (`self.CharacterMovement`))
  (`PrimitiveComponent.SetCollisionEnabled` (`self.CapsuleComponent`) "NoCollision")
  (`self.Increase Kills`))

(fn `Increase Kills`
  (bind _asbp_soldier_01 (cast `/Game/Blueprints/Pawns/BP_Soldier_01` (`GameplayStatics.GetPlayerCharacter` 0)))
  (`/Engine/EditorBlueprintResources/StandardMacros.IncrementInt` (`/Game/Blueprints/Pawns/BP_Soldier_01.Kills` _asbp_soldier_01)))

(fn `IsAlive`
  (returns (ReturnValue :type Boolean))
  (return (not (`self.Dead`))))

(fn `IsAttacking`
  (returns (ReturnValue :type Boolean))
  (return (`AnimInstance.Montage_IsPlaying` (`SkeletalMeshComponent.GetAnimInstance` (`self.Mesh`)) "/Game/Characters/Enemy_Great_Spider/Animations/SpiderAttack_01.SpiderAttack_01")))

(fn `IsAttackRange`
  (returns (ReturnValue :type Boolean))
  (return (>= (`self.AttackRange`) (`self.GetDistanceTo` (`GameplayStatics.GetPlayerCharacter` 0)))))

(fn `UserConstructionScript`)